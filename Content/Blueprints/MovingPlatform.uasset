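; Moving platform Blueprint that sweeps its Platform component between the world locations of its Start and End components.
; BeginPlay caches both locations and scales the PlatformMovement timeline's play rate by the inverse of MovementDuration.
; Each OnActivation call alternates the timeline between play and reverse through a FlipFlop, with the Movement track driving the position lerp.
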(event `self.ReceiveBeginPlay`
  ;[1 1 1] Set Start & End Locations
  (set `self.startLocation` (`SceneComponent.K2_GetComponentLocation` (`self.Start`)))
  (set `self.endLocation` (`SceneComponent.K2_GetComponentLocation` (`self.End`)))
  (`TimelineComponent.SetPlayRate` (`self.Platform Movement`) (/ 1.0 (`self.MovementDuration`))))

(event `On Activation`
  ;[1 1 1] Platform Movement
  (`/Engine/EditorBlueprintResources/StandardMacros.FlipFlop`
    (:`A`
      (bind (_direction _movement) (`Timeline|Platform Movement` :!label _label)
        (:`Update`
          (`SceneComponent.K2_SetWorldLocation` (`self.Platform`) (`KismetMathLibrary.VLerp` (`self.startLocation`) (`self.endLocation`) _movement) true false))))
    (:`B`
      (goto _label :!via `Reverse`))))

(fn `UserConstructionScript`)