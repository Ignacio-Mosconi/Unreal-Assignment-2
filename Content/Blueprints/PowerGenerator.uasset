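; PowerGenerator is an interactable actor that switches a set of rect lights on and off.
; Its Box overlap enables input for player controller 0 on entry and disables it on exit, without checking which actor overlaps.
; While input is enabled, pressing E loops over the RectLights array, toggles each light component's visibility and flips the IsOn flag inside the loop.
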(event `self.Box.OnComponentBeginOverlap`
  (params (OverlappedComponent :type "PrimitiveComponent Object Reference") (OtherActor :type "Actor Object Reference") (OtherComp :type "PrimitiveComponent Object Reference") (OtherBodyIndex :type Integer) (bFromSweep :type Boolean) (SweepResult :type "HitResult Structure (by ref)"))
  (`self.EnableInput` (`GameplayStatics.GetPlayerController` 0)))

(event `Key|E`
  (params (Key :type "Key Structure"))
  (:`Pressed`
    (if (`self.isOn`)
      (for _array_element (`self.RectLights`)
        (`SceneComponent.ToggleVisibility` (`RectLight.RectLightComponent` _array_element) false)
        (set `self.isOn` false))
      (else
        (for _array_element_2 (`self.RectLights`)
          (`SceneComponent.ToggleVisibility` (`RectLight.RectLightComponent` _array_element_2) false)
          (set `self.isOn` true))))))

(event `self.Box.OnComponentEndOverlap`
  (params (OverlappedComponent :type "PrimitiveComponent Object Reference") (OtherActor :type "Actor Object Reference") (OtherComp :type "PrimitiveComponent Object Reference") (OtherBodyIndex :type Integer))
  (`self.DisableInput` (`GameplayStatics.GetPlayerController` 0)))

(fn `UserConstructionScript`)