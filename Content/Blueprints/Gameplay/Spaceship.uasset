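; Spaceship is an interactable end-of-level actor that returns the player to the main menu.
; A Box overlap enables the actor's input and shows an interaction prompt through CustomHUD, while leaving the box disables input and hides it.
; Pressing E while input is enabled opens the MainMenu level.
; Neither overlap event checks which actor triggered it.
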(event `self.Box.OnComponentEndOverlap`
  (params (OverlappedComponent :type "PrimitiveComponent Object Reference") (OtherActor :type "Actor Object Reference") (OtherComp :type "PrimitiveComponent Object Reference") (OtherBodyIndex :type Integer))
  (bind _returnvalue (`GameplayStatics.GetPlayerController` 0))
  ;[1 1 1] HUD Display & Input Enable
  (`self.DisableInput` _returnvalue)
  ;[1 1 1] Change Prompt Text
  (bind _ascustom_hud (cast `/Game/Blueprints/UI/CustomHUD` (`PlayerController.GetHUD` _returnvalue)))
  (`/Game/Blueprints/UI/CustomHUD.Display Prompt` _ascustom_hud false ""))

(event `self.Box.OnComponentBeginOverlap`
  (params (OverlappedComponent :type "PrimitiveComponent Object Reference") (OtherActor :type "Actor Object Reference") (OtherComp :type "PrimitiveComponent Object Reference") (OtherBodyIndex :type Integer) (bFromSweep :type Boolean) (SweepResult :type "HitResult Structure (by ref)"))
  (bind _returnvalue (`GameplayStatics.GetPlayerController` 0))
  ;[1 1 1] HUD Display & Input Enable
  (`self.EnableInput` _returnvalue)
  ;[1 1 1] Change Prompt Text
  (bind _ascustom_hud (cast `/Game/Blueprints/UI/CustomHUD` (`PlayerController.GetHUD` _returnvalue)))
  (`/Game/Blueprints/UI/CustomHUD.Display Prompt` _ascustom_hud true (`self.InteractionText`)))

(event `Key|E`
  (params (Key :type "Key Structure"))
  ;[1 1 1] End Level
  (:`Pressed`
    (`GameplayStatics.OpenLevel` "MainMenu")))

(fn `UserConstructionScript`)