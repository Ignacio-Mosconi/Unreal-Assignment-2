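; AshTrigger is a trigger volume that swaps ash particle effects while something overlaps its Box.
; On begin overlap it hides the main particle system and shows every system in the SmallParticleSystems array.
; On end overlap it reverses this, using root component visibility without propagating to children.
; The overlapping actor is not filtered or counted, so any overlap toggles the effects.
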(event `self.Box.OnComponentBeginOverlap`
  (params (OverlappedComponent :type "PrimitiveComponent Object Reference") (OtherActor :type "Actor Object Reference") (OtherComp :type "PrimitiveComponent Object Reference") (OtherBodyIndex :type Integer) (bFromSweep :type Boolean) (SweepResult :type "HitResult Structure (by ref)"))
  (`SceneComponent.SetVisibility` (`Actor.RootComponent` (`self.MainParticleSystem`)) false false)
  (for _array_element (`self.SmallParticleSystems`)
    (`SceneComponent.SetVisibility` (`Actor.RootComponent` _array_element) true false)))

(event `self.Box.OnComponentEndOverlap`
  (params (OverlappedComponent :type "PrimitiveComponent Object Reference") (OtherActor :type "Actor Object Reference") (OtherComp :type "PrimitiveComponent Object Reference") (OtherBodyIndex :type Integer))
  (`SceneComponent.SetVisibility` (`Actor.RootComponent` (`self.MainParticleSystem`)) true false)
  (for _array_element (`self.SmallParticleSystems`)
    (`SceneComponent.SetVisibility` (`Actor.RootComponent` _array_element) false false)))

(fn `UserConstructionScript`)