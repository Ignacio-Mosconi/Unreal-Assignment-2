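; Moving stairs Blueprint that slides a Platform component between the positions of its Start and End components.
; BeginPlay caches both world locations and scales the StairsMovement timeline's play rate by the inverse of MovementDuration.
; Each OnActivation alternates through a FlipFlop between playing and reversing the timeline, whose Movement track lerps the platform's world location without sweeping.
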(event `self.ReceiveBeginPlay`
  ;[1 1 1] Set Start & End Locations
  (set `self.startLocation` (`SceneComponent.K2_GetComponentLocation` (`self.Start`)))
  (set `self.endLocation` (`SceneComponent.K2_GetComponentLocation` (`self.End`)))
  (`TimelineComponent.SetPlayRate` (`self.Stairs Movement`) (/ 1.0 (`self.MovementDuration`))))

(event `On Activation`
  ;[1 1 1] Stairs Movement
  (`/Engine/EditorBlueprintResources/StandardMacros.FlipFlop`
    (:`A`
      (bind (_direction _movement) (`Timeline|Stairs Movement` :!label _label)
        (:`Update`
          (`SceneComponent.K2_SetWorldLocation` (`self.Platform`) (`KismetMathLibrary.VLerp` (`self.startLocation`) (`self.endLocation`) _movement) false false))))
    (:`B`
      (goto _label :!via `Reverse`))))

(fn `UserConstructionScript`)