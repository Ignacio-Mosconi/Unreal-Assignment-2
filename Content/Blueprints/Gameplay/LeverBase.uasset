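; Base lever Blueprint that the player toggles with E while inside a box trigger, with an empty Activate function apparently meant for child overrides.
; Overlap events enable or disable input and update the CustomHUD prompt with activate or deactivate text.
; Each pull plays a sound, hides the prompt, disables input, and plays or reverses a timeline that rotates the handle, calling Activate when it finishes.
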(event `self.Box.OnComponentEndOverlap`
  (params (OverlappedComponent :type "PrimitiveComponent Object Reference") (OtherActor :type "Actor Object Reference") (OtherComp :type "PrimitiveComponent Object Reference") (OtherBodyIndex :type Integer))
  ;[1 1 1] Input Enable
  (set `self.isInRange` false)
  (`self.DisableInput` (`GameplayStatics.GetPlayerController` 0))
  (`self.ChangeInteractionText` :!label _label))

(event `self.Box.OnComponentBeginOverlap`
  (params (OverlappedComponent :type "PrimitiveComponent Object Reference") (OtherActor :type "Actor Object Reference") (OtherComp :type "PrimitiveComponent Object Reference") (OtherBodyIndex :type Integer) (bFromSweep :type Boolean) (SweepResult :type "HitResult Structure (by ref)"))
  ;[1 1 1] Input Enable
  (set `self.isInRange` true)
  (`self.EnableInput` (`GameplayStatics.GetPlayerController` 0))
  (goto _label))

(event `Key|E`
  (params (Key :type "Key Structure"))
  ;[1 1 1] Lever Pulling
  (:`Pressed`
    (`GameplayStatics.PlaySoundAtLocation` "/Game/Sounds/Cues/Lever_Pull_Cue.Lever_Pull_Cue" (`SceneComponent.K2_GetComponentLocation` (`self.Handle`)) (struct) 1.0 1.0 0.0 null null null)
    (bind _ascustom_hud (cast `/Game/Blueprints/UI/CustomHUD` (`PlayerController.GetHUD` (`GameplayStatics.GetPlayerController` 0))))
    (`/Game/Blueprints/UI/CustomHUD.Display Prompt` _ascustom_hud false "")
    (`self.DisableInput` null)
    (bind _output_get (set `self.hasActivated` (not (`self.hasActivated`))))
    (if _output_get
      (bind (_direction _lever_rotation) (`Timeline|Lever Rotation` :!label _label_2)
        (:`Update`
          (`SceneComponent.K2_SetRelativeRotation` (`self.Handle`) (`KismetMathLibrary.MakeRotator` _lever_rotation) false false))
        (:`Finished`
          (`self.Activate`)))
      (else
        (goto _label_2 :!via `Reverse`)))))

(fn `Activate`)

(fn `ChangeInteractionText`
  (if (`self.isInRange`)
    (if (`self.hasActivated`)
      (set `self.interactionText` (`self.deactivateText`))
      (else
        (set `self.interactionText` (`self.activateText`))))
    (else
      (set `self.interactionText` "")))
  (bind _ascustom_hud (cast `/Game/Blueprints/UI/CustomHUD` (`PlayerController.GetHUD` (`GameplayStatics.GetPlayerController` 0))))
  (`/Game/Blueprints/UI/CustomHUD.Display Prompt` _ascustom_hud (`self.isInRange`) (`self.interactionText`)))

(fn `UserConstructionScript`)