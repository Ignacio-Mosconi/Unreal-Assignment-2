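; Power generator actor that the player switches on and off with the E key to toggle a set of rect lights.
; Box overlap enables input and shows a state-dependent prompt through FirstPersonHUD; leaving disables input and clears the prompt text.
; Pressing E toggles visibility on each light in RectLights, setting IsOn and refreshing the prompt inside the loop.
; Lights are toggled relative to their current visibility, not set from IsOn.
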(event `self.Box.OnComponentEndOverlap`
  (params (OverlappedComponent :type "PrimitiveComponent Object Reference") (OtherActor :type "Actor Object Reference") (OtherComp :type "PrimitiveComponent Object Reference") (OtherBodyIndex :type Integer))
  (bind _returnvalue (`GameplayStatics.GetPlayerController` 0))
  ;[1 1 1] HUD Display & Input Enable
  (`self.DisableInput` _returnvalue)
  ;[1 1 1] Change Prompt Text
  (set `self.interactionText` "")
  (bind _asfirst_person_hud (cast `/Game/FirstPersonBP/Blueprints/FirstPersonHUD` (`PlayerController.GetHUD` _returnvalue) :!label _label))
  (`/Game/FirstPersonBP/Blueprints/FirstPersonHUD.Display Prompt` _asfirst_person_hud true (`self.interactionText`)))

(event `self.Box.OnComponentBeginOverlap`
  (params (OverlappedComponent :type "PrimitiveComponent Object Reference") (OtherActor :type "Actor Object Reference") (OtherComp :type "PrimitiveComponent Object Reference") (OtherBodyIndex :type Integer) (bFromSweep :type Boolean) (SweepResult :type "HitResult Structure (by ref)"))
  ;[1 1 1] HUD Display & Input Enable
  (`self.EnableInput` (`GameplayStatics.GetPlayerController` 0))
  (if (`self.isOn`)
    ;[1 1 1] Change Prompt Text
    (set `self.interactionText` "Press \"E\" to turn OFF the generator" :!label _label_2)
    (goto _label)
    (else
      (set `self.interactionText` "Press \"E\" to turn ON the generator" :!label _label_3)
      (goto _label))))

(event `Key|E`
  (params (Key :type "Key Structure"))
  ;[1 1 1] Switch Lights
  (:`Pressed`
    (if (`self.isOn`)
      (for _array_element (`self.RectLights`)
        (`SceneComponent.ToggleVisibility` (`RectLight.RectLightComponent` _array_element) false)
        (set `self.isOn` false)
        (goto _label_3))
      (else
        (for _array_element_2 (`self.RectLights`)
          (`SceneComponent.ToggleVisibility` (`RectLight.RectLightComponent` _array_element_2) false)
          (set `self.isOn` true)
          (goto _label_2))))))

(fn `UserConstructionScript`)