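; Lever that moves a linked Platform and shows an "E" interaction prompt matching the platform's travel direction.
; On BeginPlay, IsEndLocationLever decides which of the "bring" and "move away" texts serves as activate or deactivate prompt.
; Activate triggers the platform, waits out its MovementDuration, then re-enables input and changes the prompt only if IsInRange is set.
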(event `self.ReceiveBeginPlay`
  (if (`self.IsEndLocationLever`)
    (set `self.activateText` "Press \"E\" to bring the platform")
    (set `self.deactivateText` "Press \"E\" to move the platform away")
    (else
      (set `self.activateText` "Press \"E\" to move the platform away")
      (set `self.deactivateText` "Press \"E\" to bring the platform"))))

(event `self.Activate`
  ;[1 1 1] Platform Activation
  (`/Game/Blueprints/Gameplay/MovingPlatform.On Activation` (`self.Platform`))
  (`KismetSystemLibrary.Delay` (`/Game/Blueprints/Gameplay/MovingPlatform.MovementDuration` (`self.Platform`)))
  (if (`self.isInRange`)
    (`self.EnableInput` (`GameplayStatics.GetPlayerController` 0))
    (`self.ChangeInteractionText`)))

(fn `UserConstructionScript`)