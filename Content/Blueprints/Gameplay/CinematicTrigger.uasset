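; Trigger actor that plays a level sequence cinematic when its box is overlapped.
; On overlap it plays the sequence, disables input on player 0's character and waits for the sequence's duration.
; It then restores input and destroys itself, making it one-shot after completion; the overlap handler does not filter which actor entered.
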(event `self.Box.OnComponentBeginOverlap`
  (params (OverlappedComponent :type "PrimitiveComponent Object Reference") (OtherActor :type "Actor Object Reference") (OtherComp :type "PrimitiveComponent Object Reference") (OtherBodyIndex :type Integer) (bFromSweep :type Boolean) (SweepResult :type "HitResult Structure (by ref)"))
  (bind _returnvalue (`GameplayStatics.GetPlayerCharacter` 0))
  (bind _returnvalue_2 (`GameplayStatics.GetPlayerController` 0))
  (`MovieSceneSequencePlayer.Play` (`LevelSequenceActor.SequencePlayer` (`self.Cinematic`)))
  (`self.DisableInput` _returnvalue _returnvalue_2)
  (`KismetSystemLibrary.Delay` (`TimeManagementBlueprintLibrary.Conv_QualifiedFrameTimeToSeconds` (`MovieSceneSequencePlayer.GetDuration` (`LevelSequenceActor.SequencePlayer` (`self.Cinematic`)))))
  (`self.EnableInput` _returnvalue _returnvalue_2)
  (`self.K2_DestroyActor`))

(fn `UserConstructionScript`)