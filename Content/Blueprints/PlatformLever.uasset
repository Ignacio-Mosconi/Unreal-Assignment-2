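; An interactable lever that the player pulls with E to bring a platform over or move it away.
; A box trigger toggles player input and shows a HUD prompt matching the lever's state.
; Each press clears the prompt, disables input and plays or reverses a timeline that rotates the handle.
; On finish it activates the platform, waits out its movement, then restores input and prompt if the player is in range.
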(event `self.Box.OnComponentEndOverlap`
  (params (OverlappedComponent :type "PrimitiveComponent Object Reference") (OtherActor :type "Actor Object Reference") (OtherComp :type "PrimitiveComponent Object Reference") (OtherBodyIndex :type Integer))
  (bind _returnvalue (`GameplayStatics.GetPlayerController` 0))
  ;[1 1 1] Input Enable
  (set `self.isInRange` false)
  (`self.DisableInput` _returnvalue)
  ;[1 1 1] Display Prompt
  (set `self.interactionText` "" :!label _label)
  (bind _asfirst_person_hud (cast `/Game/FirstPersonBP/Blueprints/FirstPersonHUD` (`PlayerController.GetHUD` _returnvalue) :!label _label_2))
  (`/Game/FirstPersonBP/Blueprints/FirstPersonHUD.Display Prompt` _asfirst_person_hud true (`self.interactionText`)))

(event `self.Box.OnComponentBeginOverlap`
  (params (OverlappedComponent :type "PrimitiveComponent Object Reference") (OtherActor :type "Actor Object Reference") (OtherComp :type "PrimitiveComponent Object Reference") (OtherBodyIndex :type Integer) (bFromSweep :type Boolean) (SweepResult :type "HitResult Structure (by ref)"))
  ;[1 1 1] Input Enable
  (set `self.isInRange` true)
  (`self.EnableInput` (`GameplayStatics.GetPlayerController` 0))
  (if (`self.hasActivated`)
    ;[1 1 1] Display Prompt
    (set `self.interactionText` "Press \"E\" to move the platform away" :!label _label_3)
    (goto _label_2)
    (else
      (set `self.interactionText` "Press \"E\" to bring the platform" :!label _label_4)
      (goto _label_2))))

(event `Key|E`
  (params (Key :type "Key Structure"))
  ;[1 1 1] Lever Pulling
  (:`Pressed`
    (`self.DisableInput` null)
    (`|ExecutionSequence`
      (:`then_0`
        (goto _label))
      (:`then_1`
        (if (`self.hasActivated`)
          (set `self.hasActivated` false)
          (bind (_direction _lever_rotation) (`Timeline|Lever Rotation` :!via `Reverse` :!label _label_5)
            (:`Update`
              (`SceneComponent.K2_SetRelativeRotation` (`self.Handle`) (`KismetMathLibrary.MakeRotator` _lever_rotation) false false))
            (:`Finished`
              (`/Game/Blueprints/MovingPlatform.On Activation` (`self.Platform`))
              (`KismetSystemLibrary.Delay` (`/Game/Blueprints/MovingPlatform.MovementDuration` (`self.Platform`)))
              (if (`self.isInRange`)
                (`self.EnableInput` (`GameplayStatics.GetPlayerController` 0))
                (if (`self.hasActivated`)
                  (goto _label_3)
                  (else
                    (goto _label_4))))))
          (else
            (set `self.hasActivated` true)
            (goto _label_5)))))))

(fn `UserConstructionScript`)